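; Camera pawn for the vehicle game that provides an animated vertical camera move and a fixed car selection viewpoint.
; On BeginPlay, unless IsCarPawn is set, it caches the camera's world location and plays a timeline that offsets the actor's height from that point.
; MovetoCar calls CarSelectionPosition, which teleports the pawn to a hardcoded location and yaw for car selection.
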(event Custom|Move%20to%20Car
  (CallFunction|CarSelectionPosition))

(event EventBeginPlay
  (if (not (Variables|Default|GetIsCarPawn))
    (Variables|Default|SetPawnLocation (Transformation|GetWorldLocation (Variables|Default|GetCamera self)))
    (bind _newtrack_0 (Timeline|Timeline_0 Play)
      (:Update
        (Transformation|SetActorLocation (Math|Vector|MakeVector (.X (Math|Vector|BreakVector (Variables|Default|GetPawnLocation))) (.Y (Math|Vector|BreakVector (Variables|Default|GetPawnLocation))) (+ _newtrack_0 (.Z (Math|Vector|BreakVector (Variables|Default|GetPawnLocation))))) false false)))))

(event Collision|EventActorBeginOverlap
  (params (OtherActor :type Actor%20Object%20Reference)))

(event EventTick
  (params (DeltaSeconds :type Float%20%28single-precision%29)))

(fn ConstructionScript)

(fn CarSelectionPosition
  (Transformation|SetActorTransform (Math|Transform|MakeTransform (Math|Vector|MakeVector 84.0 289.0 2537.0) (Math|Rotator|MakeRotator 0.0 0.0 -129.999939)) false true)
  (return))