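; BP_Fireball is a physics-driven projectile that hurtles toward Earth and bursts on impact.
; BeginPlay pushes its sphere toward the world origin with an impulse scaled by its distance, and caches the first Planet-tagged actor.
; Hitting an Earth-tagged actor spawns an enlarged explosion, destroys the fireball and spawns BP_FireballOnEarth slightly below.
; That actor's roll and pitch are approximated linearly from the impact position and the planet sphere's bounds radius.
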(event EventBeginPlay
  ;[1 1 1] Impulse towards Earth
  (Physics|AddImpulse (Variables|Default|GetSphere) (* (Transformation|GetActorLocation) -7) "None" false)
  (bind _outactors (Actor|GetAllActorswithTag "Planet"))
  (Variables|Default|SetPlanet (Utilities|Array|Get(acopy) _outactors)))

(event Collision|EventActorBeginOverlap
  (params (OtherActor :type Actor%20Object%20Reference)))

(event EventTick
  (params (DeltaSeconds :type Float%20%28single-precision%29)))

(event Collision|EventHit
  (params (MyComp :type Primitive%20Component%20Object%20Reference) (Other :type Actor%20Object%20Reference) (OtherComp :type Primitive%20Component%20Object%20Reference) (bSelfMoved :type Boolean) (HitLocation :type Vector :default "0, 0, 0") (HitNormal :type Vector :default "0, 0, 0") (NormalImpulse :type Vector :default "0, 0, 0") (Hit :type Hit%20Result%20Structure%20%28by%20ref%29))
  (if (Actor|ActorHasTag Other "Earth")
    (CallFunction|SpawnFireballonEarth)))

(fn ConstructionScript)

(fn SpawnFireballonEarth
  (bind _output_get (Variables|Default|SetActorTransform (Transformation|GetActorTransform)))
  ;[1 1 1] Spawn Effect
  (Game|SpawnActorfromClass "/Game/StarterContent/Blueprints/Blueprint_Effect_Explosion.Blueprint_Effect_Explosion_C" (Math|Transform|MakeTransform (.Location (Math|Transform|BreakTransform _output_get)) (.Rotation (Math|Transform|BreakTransform _output_get)) (* (.Scale (Math|Transform|BreakTransform _output_get)) 2.5)) "Undefined" 0 0)
  (Actor|DestroyActor)
  (bind _asbp_planet (Utilities|Casting|CastToBP_Planet (Variables|Default|GetPlanet)))
  ;[1 1 1] Spawn FireballOnEarth
  (Game|SpawnActorfromClass "/Game/VehicleAdvBP/Blueprints/BP_FireballOnEarth.BP_FireballOnEarth_C" (Math|Transform|MakeTransform (Math|Vector|MakeVector (.X (Math|Vector|BreakVector (.Location (Math|Transform|BreakTransform _output_get)))) (.Y (Math|Vector|BreakVector (.Location (Math|Transform|BreakTransform _output_get)))) (- (.Z (Math|Vector|BreakVector (.Location (Math|Transform|BreakTransform _output_get)))) 5e+01)) (Math|Rotator|MakeRotator (* 180 (* (/ (- (.Y (Math|Vector|BreakVector (.Location (Math|Transform|BreakTransform _output_get)))) (.SphereRadius (Collision|GetComponentBounds (Variables|/Game/VehicleAdvBP/Blueprints/BP_Planet.BP_Planet_C|GetSphere _asbp_planet)))) (* 2 (.SphereRadius (Collision|GetComponentBounds (Variables|/Game/VehicleAdvBP/Blueprints/BP_Planet.BP_Planet_C|GetSphere _asbp_planet))))) -1.0)) (* 180 (* (/ (- (.Z (Math|Vector|BreakVector (.Location (Math|Transform|BreakTransform _output_get)))) (.SphereRadius (Collision|GetComponentBounds (Variables|/Game/VehicleAdvBP/Blueprints/BP_Planet.BP_Planet_C|GetSphere _asbp_planet)))) (* 2 (.SphereRadius (Collision|GetComponentBounds (Variables|/Game/VehicleAdvBP/Blueprints/BP_Planet.BP_Planet_C|GetSphere _asbp_planet))))) -1.0)) 0.0) (.Scale (Math|Transform|BreakTransform _output_get))) "Undefined" 0 0)
  (return))