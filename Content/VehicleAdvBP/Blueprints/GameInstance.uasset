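; Game instance that runs the game's front-end flow: main menu, car selection, options, level start and quit.
; Each show event creates its widget once, caches it, adds it to the viewport and switches to UI-only input with a visible cursor.
; The car menu also possesses the CameraPawn tagged Camera2.
; BeginGame stores the selected car on the instance, opens Level1 and sets game-only input.
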(event Custom|ShowOptionsMenu
  (bind _returnvalue (Game|GetPlayerController 0))
  (Utilities|IsValid (Variables|Default|GetGameOptions)
    (:Is%20Valid
      _)
    (:Is%20Not%20Valid
      (bind _returnvalue_2 (UserInterface|CreateWidget "/Game/VehicleAdvBP/Widgets/BP_Options.BP_Options_C"))
      (bind _output_get (Variables|Default|SetGameOptions _returnvalue_2))))
  (UserInterface|Viewport|AddtoViewport (Variables|Default|GetGameOptions) 0)
  (Input|SetInputModeUIOnly _returnvalue (Variables|Default|GetGameOptions) "DoNotLock")
  (Variables|/Script/Engine.PlayerController|SetbShowMouseCursor _returnvalue true))

(event Custom|ShowGameCarMenu
  (bind _returnvalue (Game|GetPlayerController 0))
  (Utilities|IsValid (Variables|Default|GetGame%20Car%20Menu)
    (:Is%20Valid
      _)
    (:Is%20Not%20Valid
      (bind _returnvalue_2 (UserInterface|CreateWidget "/Game/VehicleAdvBP/Widgets/BP_CarMenu.BP_CarMenu_C"))
      (bind _output_get (Variables|Default|SetGame%20Car%20Menu _returnvalue_2))))
  (UserInterface|Viewport|AddtoViewport (Variables|Default|GetGame%20Car%20Menu) 0)
  (CallFunction|SwitchtoCarCameraPawn)
  (Input|SetInputModeUIOnly _returnvalue (Variables|Default|GetGame%20Car%20Menu) "DoNotLock")
  (Variables|/Script/Engine.PlayerController|SetbShowMouseCursor _returnvalue true))

(event Custom|QuitGame
  (Game|QuitGame 0 "Quit" false))

(event Custom|ShowGameMenu
  (bind _returnvalue (Game|GetPlayerController 0))
  (Utilities|IsValid (Variables|Default|GetGameMenu)
    (:Is%20Valid
      _)
    (:Is%20Not%20Valid
      (bind _returnvalue_2 (UserInterface|CreateWidget "/Game/VehicleAdvBP/Widgets/BP_Menu.BP_Menu_C"))
      (bind _output_get (Variables|Default|SetGameMenu _returnvalue_2))))
  (UserInterface|Viewport|AddtoViewport _output_get 0)
  (Input|SetInputModeUIOnly _returnvalue (Variables|Default|GetGameMenu) "DoNotLock")
  (Variables|/Script/Engine.PlayerController|SetbShowMouseCursor _returnvalue true))

(event Custom|BeginGame
  (params (car :type Actor%20Class%20Reference))
  (Variables|Default|SetselectedCar car)
  (Game|OpenLevel(byName) "Level1")
  (Input|SetInputModeGameOnly (Game|GetPlayerController 0)))

(fn SwitchtoCarCameraPawn
  (bind _outactors (Actor|GetAllActorsOfClasswithTag "/Game/VehicleAdvBP/Blueprints/Pawns/CameraPawn.CameraPawn_C" "Camera2"))
  (bind _ascamera_pawn (Utilities|Casting|CastToCameraPawn (Utilities|Array|Get(acopy) _outactors)))
  (Pawn|Possess (Game|GetPlayerController 0) _ascamera_pawn)
  (return))